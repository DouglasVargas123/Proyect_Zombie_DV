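; Shooting component for the third-person character that runs a preview hitscan from the follow camera while the shoot input is held.
; BeginPlay caches the owning character's camera, and IA_Shoot toggles a shoot-mode flag that Tick checks.
; Each active tick line-traces forward on the Visibility channel with debug drawing, sending OnCollisionEnterMessage to hit actors that implement BPI_Collision.
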(event Custom|PreviewShoot
  (bind _camera (Variables|Default|GetCamera))
  (bind _returnvalue (Transformation|GetWorldTransform _camera))
  (bind (_outhit _returnvalue_2) (Collision|LineTraceByChannel (.location _returnvalue) (+ (.location _returnvalue) (* (Math|Vector|GetForwardVector (.rotation _returnvalue)) (Variables|Default|GetShootDistance))) "TraceTypeQuery1" false 0 "ForDuration"))
  (if _returnvalue_2
    (if (Utilities|DoesObjectImplementInterface (.HitActor (Collision|BreakHitResult _outhit)) "/Game/00_Blueprints/02_Blueprint_Interface/BPI_Collision.BPI_Collision_C")
      (Class|BPICollision|OnCollisionEnter(Message) (.HitActor (Collision|BreakHitResult _outhit))))))

(event Input|EnhancedActionEvents|EnhancedInputActionIA_Shoot
  (params (ActionValue :type Boolean) (ElapsedSeconds :type Float%20%28double-precision%29) (TriggeredSeconds :type Float%20%28double-precision%29) (InputAction :type Input%20Action%20Object%20Reference :default "/Game/00_Blueprints/00_ThirdPerson/Input/Actions/IA_Shoot.IA_Shoot"))
  (:Started
    (Variables|Default|SetinShootMode? true))
  (:Completed
    (Variables|Default|SetinShootMode? false)))

(event EventBeginPlay
  (bind _asbp_third_person_character (Utilities|Casting|CastToBP_ThirdPersonCharacter (Components|GetOwner)))
  (Variables|Default|SetCamera (Variables|/Game/00_Blueprints/00_ThirdPerson/Blueprints/BP_ThirdPersonCharacter.BP_ThirdPersonCharacter_C|GetFollowCamera _asbp_third_person_character))
  (Variables|Default|SetAs%20BP%20Third%20Person%20Character _asbp_third_person_character))

(event EventTick
  (params (DeltaSeconds :type Float%20%28single-precision%29))
  (if (Variables|Default|GetinShootMode?)
    (CallFunction|PreviewShoot)))