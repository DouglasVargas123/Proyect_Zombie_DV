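; BP_Door is a door that consumes a key item from the player's inventory and can swing open.
; OnCollisionEnter casts the player pawn to BP_ThirdPersonCharacter and removes the key through its inventory component, without checking the result.
; The separate Abrir event plays the AnimacionPuerta timeline to drive Puerta's relative yaw, printing a debug string each update.
; Nothing in this Blueprint calls Abrir, so key removal does not open the door here.
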(event Custom|Abrir
  (bind _valor_rotacion (Timeline|Animacion%20Puerta Play)
    (:Update
      (Transformation|SetRelativeRotation (Variables|Default|GetPuerta) (Math|Rotator|MakeRotator 0.0 0.0 _valor_rotacion) false false)
      (Development|PrintString "Rotado"))))

(event EventOnCollisionEnter
  (bind _asbp_third_person_character (Utilities|Casting|CastToBP_ThirdPersonCharacter (Game|Player|GetPlayerPawn 0)))
  (Default|RemovefromInventory (Variables|/Game/00_Blueprints/00_ThirdPerson/Blueprints/BP_ThirdPersonCharacter.BP_ThirdPersonCharacter_C|GetBP_Inventory_Component _asbp_third_person_character) (Variables|Default|GetKey) (Variables|Default|GetQuantity%20To%20Remove)))

(fn ConstructionScript)