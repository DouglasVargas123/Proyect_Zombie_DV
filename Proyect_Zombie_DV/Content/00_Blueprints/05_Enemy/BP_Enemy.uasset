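; BP_Enemy is an enemy actor that destroys itself when its collision event fires.
; The event first calls CalcularVida, which sets VidaActual (current health) to 1.0 minus its current value and prints the result if it is zero or below.
; Destruction follows every collision regardless of the resulting health, and the construction script is empty.
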(event EventOnCollisionEnter
  (CallFunction|CalcularVida)
  (Actor|DestroyActor self))

(fn ConstructionScript)

(fn CalcularVida
  (Variables|Default|SetVidaActual (- 1.0 (Variables|Default|GetVidaActual)))
  (if (<= (Variables|Default|GetVidaActual) 0.0)
    (Development|PrintString (Utilities|String|ToString(Float) (Variables|Default|GetVidaActual)))))