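; Inventory component that stores items in a map from item name to quantity.
; AddToInventory adds to an existing count or creates a new entry.
; RemoveFromInventory checks stock, then lowers the count or deletes the entry, printing debug messages on deletion or failure.
; Deleting any entry also calls Abrir (open) on the BP_Door found through GetActorOfClass, coupling the inventory to that door.
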(event EventBeginPlay)

(event EventTick
  (params (DeltaSeconds :type Float%20%28single-precision%29)))

(fn AddtoInventory
  (params (Name%20Item%20To%20Add :type Name%20%28by%20ref%29) (Quantity%20to%20Add :type Integer%20%28by%20ref%29))
  (bind _inventory (Variables|Default|GetInventory))
  (bind (_value _returnvalue) (Utilities|Map|Find _inventory Name%20Item%20To%20Add))
  (if _returnvalue
    (Utilities|Map|Add (Variables|Default|GetInventory) Name%20Item%20To%20Add (+ Quantity%20to%20Add _value))
    (else
      (Utilities|Map|Add (Variables|Default|GetInventory) Name%20Item%20To%20Add Quantity%20to%20Add))))

(fn RemovefromInventory
  (params (Item%20to%20remove :type Name%20%28by%20ref%29) (Quantity%20to%20remove :type Integer%20%28by%20ref%29))
  (bind _inventory (Variables|Default|GetInventory))
  (bind (_value _returnvalue) (Utilities|Map|Find _inventory Item%20to%20remove))
  (bind _returnvalue_2 (- _value Quantity%20to%20remove))
  (if _returnvalue
    (if (<= Quantity%20to%20remove _value)
      (if (<= _returnvalue_2 0)
        (Utilities|Map|Remove (Variables|Default|GetInventory) Item%20to%20remove)
        (Development|PrintString "Item Borrado")
        (bind _returnvalue_3 (Actor|GetActorOfClass "/Game/00_Blueprints/03_Puerta/BP_Door.BP_Door_C"))
        (Default|Abrir _returnvalue_3)
        (else
          (Utilities|Map|Add (Variables|Default|GetInventory) Item%20to%20remove _returnvalue_2)))
      (else
        (Development|PrintString "No tengo suficiente :(")))
    (else
      (Development|PrintString "No item :("))))